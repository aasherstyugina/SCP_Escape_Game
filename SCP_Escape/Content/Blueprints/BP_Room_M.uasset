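; BP_Room_M is a room Blueprint, extending a parent class, that configures its entrance and two exit doors when play begins.
; After the parent BeginPlay, it moves DoorEnter to a fixed relative location.
; It then casts the DoorExit1 and DoorExit2 child actors to BP_Door, giving each a reference to this room and flagging only DoorExit1 as the first door.
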(event EventBeginPlay
  (|CallParentFunction)
  (Transformation|SetRelativeLocation (Variables|Default|GetDoorEnter) "100.000000,1500.000000,50.000000" false false)
  (bind _asbp_door (Utilities|Casting|CastToBP_Door (Variables|/Script/Engine.ChildActorComponent|GetChildActor (Variables|Default|GetDoorExit1))))
  (Variables|/Game/Blueprints/BP_Door.BP_Door_C|SetRoom _asbp_door self)
  (Variables|/Game/Blueprints/BP_Door.BP_Door_C|SetIsFirstDoor _asbp_door true)
  (bind _asbp_door_2 (Utilities|Casting|CastToBP_Door (Variables|/Script/Engine.ChildActorComponent|GetChildActor (Variables|Default|GetDoorExit2))))
  (Variables|/Game/Blueprints/BP_Door.BP_Door_C|SetRoom _asbp_door_2 self)
  (Variables|/Game/Blueprints/BP_Door.BP_Door_C|SetIsFirstDoor _asbp_door_2 false))

(event Collision|EventActorBeginOverlap
  (params (OtherActor :type Actor%20Object%20Reference))
  (|CallParentFunction OtherActor) ; This node is disabled and will not be called.\nDrag off pins to build functionality.
)

(event EventTick
  (params (DeltaSeconds :type Float%20%28single-precision%29))
  (|CallParentFunction DeltaSeconds) ; This node is disabled and will not be called.\nDrag off pins to build functionality.
)

(fn ConstructionScript
  (|CallParentFunction))