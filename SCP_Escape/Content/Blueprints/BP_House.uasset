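; House Blueprint that randomly wires nine child-actor BP_Room rooms into a maze at BeginPlay and moves the player to the start room's entrance.
; It picks start and end rooms, then chains every room between them in random order through Exit1 or Exit2.
; Each non-end room's spare exit then links to a random room from roughly the first two-thirds of that path, creating loops and backtracks.
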(event EventBeginPlay
  (bind _startroom (Variables|Default|GetStartRoom))
  (bind _rooms (Variables|Default|GetRooms))
  (bind _output (Utilities|Array|Get(acopy) _rooms _startroom))
  (CallFunction|SetRoomsArray)
  (CallFunction|SetStartRoom)
  (Transformation|SetActorLocation (Game|GetPlayerCharacter 0) (+ (.Location (Math|Transform|BreakTransform (Transformation|GetRelativeTransform (Variables|/Game/Blueprints/BP_Room.BP_Room_C|GetDoorEnter _output)))) (.Location (Math|Transform|BreakTransform (Transformation|GetActorTransform _output)))) false false)
  (CallFunction|SetEndRoom)
  (CallFunction|SetPath)
  (for (_array_element _array_index) (Variables|Default|GetInPath)
    (Development|PrintString (Utilities|String|BuildString(Integer) (Utilities|String|ToString(Integer) _array_index) " is a " _array_element)))
  (CallFunction|SetOtherDoors))

(fn ConstructionScript)

(fn SetStartRoom
  (bind _index (CallFunction|GetRoomNotinPath))
  (Variables|Default|SetStartRoom _index)
  (Utilities|Array|Add (Variables|Default|GetInPath) _index)
  (Development|PrintString (Utilities|String|BuildString(Integer) "Start: " "" _index)))

(fn SetEndRoom
  (bind _index (CallFunction|GetRoomNotinPath))
  (Variables|Default|SetEndRoom _index)
  (Development|PrintString (Utilities|String|BuildString(Integer) "End: " "" _index)))

(fn SetPath
  (bind _endroom (Variables|Default|GetEndRoom))
  (bind _rooms (Variables|Default|GetRooms))
  (bind _output (Utilities|Array|Get(acopy) _rooms _endroom))
  (Variables|Default|SetLastRoom (Variables|Default|GetStartRoom))
  (while (!= (Utilities|Array|Length (Variables|Default|GetInPath)) (- (Utilities|Array|Length (Variables|Default|GetRooms)) 1))
    (bind _index (CallFunction|GetRoomNotinPath))
    (if (Math|Random|RandomBool)
      (Variables|/Game/Blueprints/BP_Room.BP_Room_C|SetExit1 (Utilities|Array|Get(acopy) (Variables|Default|GetRooms) (Variables|Default|GetLastRoom)) (Utilities|Array|Get(acopy) (Variables|Default|GetRooms) _index))
      (else
        (Variables|/Game/Blueprints/BP_Room.BP_Room_C|SetExit2 (Utilities|Array|Get(acopy) (Variables|Default|GetRooms) (Variables|Default|GetLastRoom)) (Utilities|Array|Get(acopy) (Variables|Default|GetRooms) _index))))
    (Variables|Default|SetLastRoom _index)
    (Utilities|Array|Add (Variables|Default|GetInPath) _index))
  (if (Math|Random|RandomBool)
    (Variables|/Game/Blueprints/BP_Room.BP_Room_C|SetExit1 (Utilities|Array|Get(acopy) (Variables|Default|GetRooms) (Variables|Default|GetLastRoom)) _output)
    (else
      (Variables|/Game/Blueprints/BP_Room.BP_Room_C|SetExit2 (Utilities|Array|Get(acopy) (Variables|Default|GetRooms) (Variables|Default|GetLastRoom)) _output)))
  (Utilities|Array|Add (Variables|Default|GetInPath) (Variables|Default|GetEndRoom)))

(fn SetRoomsArray
  (bind _asbp_room (Utilities|Casting|CastToBP_Room (Variables|/Script/Engine.ChildActorComponent|GetChildActor (Variables|Default|GetBP_Room_1))))
  (bind _asbp_room_2 (Utilities|Casting|CastToBP_Room (Variables|/Script/Engine.ChildActorComponent|GetChildActor (Variables|Default|GetBP_Room_2))))
  (bind _asbp_room_3 (Utilities|Casting|CastToBP_Room (Variables|/Script/Engine.ChildActorComponent|GetChildActor (Variables|Default|GetBP_Room_3))))
  (bind _asbp_room_4 (Utilities|Casting|CastToBP_Room (Variables|/Script/Engine.ChildActorComponent|GetChildActor (Variables|Default|GetBP_Room_4))))
  (bind _asbp_room_5 (Utilities|Casting|CastToBP_Room (Variables|/Script/Engine.ChildActorComponent|GetChildActor (Variables|Default|GetBP_Room_5))))
  (bind _asbp_room_6 (Utilities|Casting|CastToBP_Room (Variables|/Script/Engine.ChildActorComponent|GetChildActor (Variables|Default|GetBP_Room_6))))
  (bind _asbp_room_7 (Utilities|Casting|CastToBP_Room (Variables|/Script/Engine.ChildActorComponent|GetChildActor (Variables|Default|GetBP_Room_7))))
  (bind _asbp_room_8 (Utilities|Casting|CastToBP_Room (Variables|/Script/Engine.ChildActorComponent|GetChildActor (Variables|Default|GetBP_Room_8))))
  (bind _asbp_room_9 (Utilities|Casting|CastToBP_Room (Variables|/Script/Engine.ChildActorComponent|GetChildActor (Variables|Default|GetBP_Room_9))))
  (Variables|Default|SetRooms (Utilities|Array|MakeArray _asbp_room _asbp_room_2 _asbp_room_3 _asbp_room_4 _asbp_room_5 _asbp_room_6 _asbp_room_7 _asbp_room_8 _asbp_room_9)))

(fn GetRoomNotinPath
  (while true
    (Variables|Default|SetBoolValue false)
    (Variables|Default|SetIntValue (Math|Random|RandomIntegerinRange 0 (- (Utilities|Array|Length (Variables|Default|GetRooms)) 1)))
    (for _array_element (Variables|Default|GetInPath)
      (if (== _array_element (Variables|Default|GetIntValue))
        (Variables|Default|SetBoolValue true)))
    (if (not (Variables|Default|GetBoolValue))
      (if (!= (Variables|Default|GetIntValue) (Variables|Default|GetEndRoom))
        (return (Variables|Default|GetIntValue))))))

(fn SetOtherDoors
  (bind _inpath (Variables|Default|GetInPath))
  (bind _rooms (Variables|Default|GetRooms))
  (bind _inpath_2 (Variables|Default|GetInPath))
  (bind _returnvalue (Utilities|Array|Length _inpath_2))
  (bind _returnvalue_2 (/ _returnvalue 3))
  (bind _returnvalue_3 (* _returnvalue_2 2))
  (bind _returnvalue_4 (Math|Random|RandomIntegerinRange 0 _returnvalue_3))
  (bind _output (Utilities|Array|Get(acopy) _inpath _returnvalue_4))
  (bind _output_2 (Utilities|Array|Get(acopy) _rooms _output))
  (for _index (range 0 (- (Utilities|Array|Length (Variables|Default|GetInPath)) 2))
    (while (== (Utilities|Array|Get(acopy) (Variables|Default|GetInPath) _index) _output)
      _)
    (Utilities|IsValid (Variables|/Game/Blueprints/BP_Room.BP_Room_C|GetExit1 (Utilities|Array|Get(acopy) (Variables|Default|GetRooms) (Utilities|Array|Get(acopy) (Variables|Default|GetInPath) _index)))
      (:Is%20Valid
        (Utilities|IsValid (Variables|/Game/Blueprints/BP_Room.BP_Room_C|GetExit2 (Utilities|Array|Get(acopy) (Variables|Default|GetRooms) (Utilities|Array|Get(acopy) (Variables|Default|GetInPath) _index)))
          (:Is%20Not%20Valid
            (Variables|/Game/Blueprints/BP_Room.BP_Room_C|SetExit2 (Utilities|Array|Get(acopy) (Variables|Default|GetRooms) (Utilities|Array|Get(acopy) (Variables|Default|GetInPath) _index)) _output_2))))
      (:Is%20Not%20Valid
        (Variables|/Game/Blueprints/BP_Room.BP_Room_C|SetExit1 (Utilities|Array|Get(acopy) (Variables|Default|GetRooms) (Utilities|Array|Get(acopy) (Variables|Default|GetInPath) _index)) _output_2)))))