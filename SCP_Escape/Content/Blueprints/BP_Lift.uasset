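; BP_Lift is a lift actor whose Platform component moves continuously up and down between fixed world-height limits.
; On BeginPlay it sets an upward offset and moves the actor to a random height within that range.
; Each Tick reverses the offset when the Platform passes either limit, then applies it as an unswept local move, so speed depends on frame rate.
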(event EventBeginPlay
  (bind _platform (Variables|Default|GetPlatform))
  (bind _returnvalue (Transformation|GetWorldLocation _platform))
  (bind (_x _y) (Math|Vector|BreakVector _returnvalue))
  (Variables|Default|SetOffset "0, 0,5.000000")
  (Transformation|SetActorLocation (Math|Vector|MakeVector _x _y (Math|Random|RandomFloatinRange 0.0 2e+02)) false false))

(event EventTick
  (params (DeltaSeconds :type Float%20%28single-precision%29))
  (bind _platform (Variables|Default|GetPlatform))
  (bind _returnvalue (Transformation|GetWorldLocation _platform))
  (bind _z (Math|Vector|BreakVector _returnvalue))
  (if (< _z 0.0)
    (Variables|Default|SetOffset "0, 0,5.000000")
    (elif (> _z 2e+02)
      (Variables|Default|SetOffset "0, 0,-5.000000")))
  (Transformation|AddLocalOffset _platform (Variables|Default|GetOffset) false false))

(fn ConstructionScript)