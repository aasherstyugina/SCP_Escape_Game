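; BP_Enemy is a simple melee enemy that chases and damages the player once it spots a pawn.
; PawnSensing sets a seeing flag, never cleared here, and calls FolloPlayer, which uses AI MoveTo toward the player.
; On arrival it applies damage and starts a delayed CanAttack cooldown, though every new FolloPlayer call resets that flag immediately.
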(event OnSeePawn(PawnSensing)
  (params (Pawn :type Pawn%20Object%20Reference))
  (Variables|Default|SetIsSeeingPlayer true)
  (CallFunction|FolloPlayer))

(event Custom|FolloPlayer
  (Variables|Default|SetCanAttack true)
  (if (Variables|Default|GetIsSeeingPlayer)
    (AI|AIMoveTo self "0, 0, 0" (Game|GetPlayerCharacter 0) 7e+01 false
      (:OnSuccess
        (if (Variables|Default|GetCanAttack)
          (Variables|Default|SetCanAttack false)
          (Development|PrintString "damaging you!!!")
          (Game|Damage|ApplyDamage (Game|GetPlayerCharacter 0) 1e+01 0 self)
          (Utilities|FlowControl|Delay 2.0)
          (Variables|Default|SetCanAttack true))))))

(event EventBeginPlay)

(event EventTick
  (params (DeltaSeconds :type Float%20%28single-precision%29)))

(fn ConstructionScript)