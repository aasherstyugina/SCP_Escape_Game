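; Door-named jumpscare ("scrimer") trigger that fires when E is pressed inside its Box.
; Box overlap enables the actor's input and opens a gate, while end overlap only disables input, leaving the gate open.
; Pressing E through the gate plays the scare sound at world origin, then briefly shows the WB_Scrimer_2 widget before removing it.
; No door movement is scripted here.
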(event OnComponentBeginOverlap(Box)
  (params (OverlappedComponent :type Primitive%20Component%20Object%20Reference) (OtherActor :type Actor%20Object%20Reference) (OtherComp :type Primitive%20Component%20Object%20Reference) (OtherBodyIndex :type Integer) (bFromSweep :type Boolean) (SweepResult :type Hit%20Result%20Structure%20%28by%20ref%29))
  (Input|EnableInput (Game|GetPlayerController 0))
  (Utilities|FlowControl|Gate true) ; enters at Open
)

(event OnComponentEndOverlap(Box)
  (params (OverlappedComponent :type Primitive%20Component%20Object%20Reference) (OtherActor :type Actor%20Object%20Reference) (OtherComp :type Primitive%20Component%20Object%20Reference) (OtherBodyIndex :type Integer))
  (Input|DisableInput (Game|GetPlayerController 0)))

(event Input|KeyboardEvents|E
  (params (Key :type Key%20Structure :default "None"))
  (:Pressed
    (Utilities|FlowControl|Gate true
      (:Exit
        (Audio|PlaySoundatLocation "/Game/Sounds/scrimer_2_sound.scrimer_2_sound" "0, 0, 0" "0, 0, 0" 1.0 1.0 0.0 0 0 0 0)
        (Utilities|FlowControl|Delay 0.3)
        (bind _returnvalue (UserInterface|CreateWidget "/Game/Widgets/WB_Scrimer_2.WB_Scrimer_2_C"))
        (UserInterface|Viewport|AddtoViewport _returnvalue 0)
        (Utilities|FlowControl|Delay 2.0)
        (Widget|RemovefromParent _returnvalue)))))

(fn ConstructionScript)